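; First-person player character Blueprint handling WASD movement, mouse look, a flashlight and limited sprinting.
; Run raises walk speed until released or until a timeline finishes, which forces walking and blocks sprinting for a short cooldown.
; The flashlight input toggles the SpotLight only when HasFlashlight is set; the Flashlight component starts hidden.
; PopupHud creates a FadeinText widget showing the string stored by Whatshouldhudsay, without adding it to the viewport here.
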(event Custom|PopupHud
  ;[1 1 1] HUD
  (bind _returnvalue (UserInterface|CreateWidget "/Game/Widget/FadeinText.FadeinText_C"))
  (Variables|/Game/Widget/FadeinText.FadeinText_C|SetTexttoshow _returnvalue (Variables|Default|GetItemAccompaniedString)))

(event EventBeginPlay
  ;[1 1 1] Flashlight
  (Rendering|SetVisibility (Variables|Default|GetFlashlight) false false))

(event Input|ActionEvents|InputActionRun
  (params (Key :type Key%20Structure :default "None"))
  ;[1 1 1] Sprinting
  (:Pressed
    (CallFunction|Sprint)
    (Timeline|Timeline_0 PlayFromStart
      (:Finished
        (CallFunction|ForceSlowdown)
        (Utilities|FlowControl|Delay 3.0)
        (Variables|Default|SetSprintRanOut false))))
  (:Released
    (CallFunction|SlowDown)))

(event Input|ActionEvents|InputActionFlashlight
  (params (Key :type Key%20Structure :default "None"))
  (bind _spotlight (Variables|Default|GetSpotLight))
  ;[1 1 1] Turn on or off
  (:Pressed
    (if (Variables|Default|GetHasFlashlight)
      (Utilities|FlowControl|FlipFlop
        (:A
          (Rendering|ToggleVisibility _spotlight false))
        (:B
          (Rendering|ToggleVisibility _spotlight false))))))

(event Input|AxisEvents|InputAxisForward/Backward
  (params (AxisValue :type Float%20%28single-precision%29))
  ;[1 1 1] Movement WASD
  (Pawn|Input|AddMovementInput (Transformation|GetActorForwardVector) AxisValue false))

(event Input|AxisEvents|InputAxisStraifeLeft/Right
  (params (AxisValue :type Float%20%28single-precision%29))
  ;[1 1 1] Movement WASD
  (Pawn|Input|AddMovementInput (Transformation|GetActorRightVector) AxisValue false))

(event Input|AxisEvents|InputAxisMouseUp/Down
  (params (AxisValue :type Float%20%28single-precision%29))
  ;[1 1 1] Rotate and turn
  (Pawn|Input|AddControllerPitchInput AxisValue))

(event Input|AxisEvents|InputAxisMouseLeft/Right
  (params (AxisValue :type Float%20%28single-precision%29))
  ;[1 1 1] Rotate and turn
  (Pawn|Input|AddControllerYawInput AxisValue))

(fn ConstructionScript)

(fn Sprint
  (if (not (Variables|Default|GetSprintRanOut))
    (Variables|/Script/Engine.CharacterMovementComponent|SetMaxWalkSpeed (Variables|Character|GetCharacterMovement) (Variables|Default|GetRunSpeed))))

(fn SlowDown
  (Variables|/Script/Engine.CharacterMovementComponent|SetMaxWalkSpeed (Variables|Character|GetCharacterMovement) (Variables|Default|GetWalk)))

(fn ForceSlowdown
  (Variables|/Script/Engine.CharacterMovementComponent|SetMaxWalkSpeed (Variables|Character|GetCharacterMovement) (Variables|Default|GetWalk))
  (Variables|Default|SetSprintRanOut true))

(fn Whatshouldhudsay
  (params (Whattosay :type String))
  (bind _output_get (Variables|Default|SetItemAccompaniedString Whattosay))
  (return _output_get))