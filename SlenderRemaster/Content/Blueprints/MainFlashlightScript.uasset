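; Flashlight Blueprint that randomly flickers a spotlight and, on BeginPlay, tells the MainMenuChar player pawn to look down.
; BlinkHandling, not called within this graph, sets a long random timer to Hardflicker, which starts a looping timer on Flicker.
; Each Flicker runs FlickerRapid, which, if CanFlicker is set, loops through delayed visibility and intensity changes with a debug print.
; The nodes that set CanFlicker are disconnected.
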(event Custom|Flicker
  (CallFunction|FlickerRapid))

(event Custom|FlickerRapid
  (if (Variables|Default|GetCanFlicker)
    (for _index (range 0 (Math|Random|RandomIntegerinRange 8 30))
      (Utilities|FlowControl|Delay (Math|Random|RandomFloatinRange 0.0 1.0))
      (Rendering|SetVisibility (Variables|Default|GetSpotLightComponent) false false)
      (Rendering|Components|Light|SetIntensity (Variables|Default|GetSpotLightComponent) (Math|Random|RandomFloatinRange 0.4 1.5))
      (Utilities|FlowControl|Delay (Math|Random|RandomFloatinRange 0.2 0.5))
      (Rendering|SetVisibility (Variables|Default|GetSpotLightComponent) true false)
      (Rendering|Components|Light|SetIntensity (Variables|Default|GetSpotLightComponent) (Math|Random|RandomFloatinRange 0.4 1.5))
      (Development|PrintString "Hello"))))

(event Custom|Hardflicker
  (Utilities|Time|SetTimerbyEvent (delegate Custom|Flicker) (Math|Random|RandomFloatinRange 0.0 5.0) true))

(event Custom|BlinkHandling
  (Utilities|Time|SetTimerbyEvent (delegate Custom|Hardflicker) (Math|Random|RandomFloatinRange 6e+01 3.6e+02)))

(event EventBeginPlay
  (bind _asmain_menu_char (Utilities|Casting|CastToMainMenuChar (Game|Player|GetPlayerPawn 0)))
  (Default|LookDown _asmain_menu_char))

(event EventTick
  (params (DeltaSeconds :type Float%20%28single-precision%29)))

(fn ConstructionScript)