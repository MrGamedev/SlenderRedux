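; Main menu character that eases its camera into a set view, then brings up the main menu.
; Each Tick interpolates MainCam's world rotation toward a hardcoded target and compares the result to the RotateTO variable within a small tolerance.
; Once they match, a DoOnce creates the Main_Menu widget, adds it to the viewport and shows the mouse cursor.
; BeginPlay and LookDown are empty.
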(event Custom|LookDown)

(event EventBeginPlay)

(event Collision|EventActorBeginOverlap
  (params (OtherActor :type Actor%20Object%20Reference)))

(event EventTick
  (params (DeltaSeconds :type Float%20%28single-precision%29))
  (bind _returnvalue (Game|GetPlayerController 0))
  (bind _maincam (Variables|Default|GetMainCam))
  (bind _returnvalue_2 (Transformation|GetWorldRotation _maincam))
  (bind _returnvalue_3 (Math|Interpolation|RInterpTo _returnvalue_2 "-10.000000,70.000092,1.000000" DeltaSeconds 0.9))
  (Transformation|SetWorldRotation (Variables|Default|GetMainCam) _returnvalue_3 false false)
  (if (Math|Rotator|Equal(Rotator) _returnvalue_3 (Variables|Default|GetRotateTO) 2.0)
    (Utilities|FlowControl|DoOnce false
      (:Completed
        (bind _returnvalue_4 (UserInterface|CreateWidget "/Game/Blueprints/Main_Menu.Main_Menu_C" _returnvalue))
        (UserInterface|Viewport|AddtoViewport _returnvalue_4 0)
        (Variables|/Script/Engine.PlayerController|SetbShowMouseCursor _returnvalue true)))))

(fn ConstructionScript)